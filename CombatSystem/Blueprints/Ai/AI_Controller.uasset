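; AI controller for BP_MasterAI pawns that runs the pawn's behavior tree and picks players as targets through AI perception.
; On possession it binds to the pawn's CombatComponent, mirroring combat toggles into the Blackboard.
; Perception updates branch on stimulus index: both handled senses target actors tagged Character.Player, but only the first clears the target when sensing fails.
; SetTargetActor writes the Blackboard Target and notifies the pawn.
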(event OnPerceptionUpdated(AIPerception)
  (params (UpdatedActors :type Array%20of%20Actor%20Object%20References))
  (CallFunction|UpdatePerception UpdatedActors))

(event Custom|OnCombatToggle
  (params (bIsCombatEnabled? :type Boolean))
  (AI|Components|Blackboard|SetValueasBool (Variables|Default|GetBlackboard) (Utilities|Name|MakeLiteralName "bCombatEnabled") bIsCombatEnabled?))

(event EventBeginPlay)

(event EventTick
  (params (DeltaSeconds :type Float%20%28single-precision%29)))

(event EventPossess
  (params (PossessedPawn :type Pawn%20Object%20Reference))
  (bind _asbp_master_ai (Utilities|Casting|CastToBP_MasterAI PossessedPawn))
  (Variables|Default|SetMaster%20AI _asbp_master_ai)
  (EventDispatchers|BindEventtoOnCombatToggled (Variables|/Game/CombatSystem/Blueprints/Ai/BP_MasterAI.BP_MasterAI_C|GetCombatComponent (Variables|Default|GetMaster%20AI)) (delegate Custom|OnCombatToggle))
  (AI|RunBehaviorTree (Variables|/Game/CombatSystem/Blueprints/Ai/BP_MasterAI.BP_MasterAI_C|GetBehaviorTree (Variables|Default|GetMaster%20AI))))

(fn ConstructionScript)

(fn UpdatePerception
  (params (PerceivedActors :type Array%20of%20Actor%20Object%20References))
  (for _array_element PerceivedActors
    (LocalVariables|SetL_SensedActor _array_element)
    (bind _info (Class|AIPerceptionComponent|GetActorsPerception (Variables|Default|GetAIPerception) (LocalVariables|GetL_SensedActor)))
    (for (_array_element_2 _array_index) (.LastSensedStimuli (Utilities|Struct|BreakActorPerceptionBlueprintInfo _info))
      (LocalVariables|SetL_AIStimilus _array_element_2)
      (switch int _array_index
        (:0
          (if (.bSuccessfullySensed (Utilities|Struct|BreakAIStimulus (LocalVariables|GetL_AIStimilus)))
            (bind _returnvalue (Class|GameplayTagBPI|HasMatchingGameplayTag(Message) (LocalVariables|GetL_SensedActor) "(TagName=\"Character.Player\")"))
            (if _returnvalue
              (CallFunction|SetTargetActor (LocalVariables|GetL_SensedActor)))
            (else
              (CallFunction|SetTargetActor))))
        (:1
          (if (.bSuccessfullySensed (Utilities|Struct|BreakAIStimulus (LocalVariables|GetL_AIStimilus)))
            (bind _returnvalue_2 (Class|GameplayTagBPI|HasMatchingGameplayTag(Message) (LocalVariables|GetL_SensedActor) "(TagName=\"Character.Player\")"))
            (if _returnvalue_2
              (CallFunction|SetTargetActor (LocalVariables|GetL_SensedActor)))))))))

(fn SetTargetActor
  (params (NewTargetActor :type Actor%20Object%20Reference))
  (AI|Components|Blackboard|SetValueasObject (Variables|Default|GetBlackboard) (Utilities|Name|MakeLiteralName "Target") NewTargetActor)
  (bind _master_ai (Variables|Default|GetMaster%20AI)
    (:then
      (Default|OnTargetSet _master_ai NewTargetActor))
    (:else)))