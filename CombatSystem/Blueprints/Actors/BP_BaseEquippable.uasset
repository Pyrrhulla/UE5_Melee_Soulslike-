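; Base actor for equippable items in the combat system, providing equip, unequip and attachment functions.
; GetItemMesh returns the static mesh component when it has a valid mesh, otherwise the skeletal one.
; OnEquipped calls AttachActor to snap the item to a named socket on the owning Character's mesh.
; As written, OnEquipped, OnUnequipped and SetIsEquipped only ever set IsEquipped to false, and unequipping does not detach.
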(event EventBeginPlay)

(event Collision|EventActorBeginOverlap
  (params (OtherActor :type Actor%20Object%20Reference)))

(event EventTick
  (params (DeltaSeconds :type Float%20%28single-precision%29)))

(fn ConstructionScript)

(fn GetItemMesh
  (Utilities|IsValid (Variables|/Script/Engine.StaticMeshComponent|GetStaticMesh (Variables|Default|GetitemStaticMesh))
    (:Is%20Valid
      (return (Variables|Default|GetitemStaticMesh)))
    (:Is%20Not%20Valid
      (return (Variables|Default|GetitemSkeletalMesh)))))

(fn OnEquipped
  (Variables|Default|SetIsEquipped? false)
  (ItemMesh|AttachActor (Variables|initialization|GetAttach%20Socket%20Name)))

(fn OnUnequipped
  (if (Variables|Default|GetIsEquipped?)
    (Variables|Default|SetIsEquipped? false)))

(fn AttachActor
  (params (SocketName :type Name))
  (Transformation|AttachComponentToComponent (Variables|/Script/Engine.Character|GetMesh (.AsCharacter (Utilities|Casting|CastToCharacter (Components|GetOwner)))) SocketName "SnapToTarget" "SnapToTarget" "SnapToTarget" true))

(fn SetIsEquipped
  (params (IsEquipped? :type Boolean))
  (Variables|Default|SetIsEquipped? false))

(fn IsEquipped
  (return (Variables|Default|GetIsEquipped?)))