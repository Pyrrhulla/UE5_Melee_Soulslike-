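; Base weapon actor for the combat system that handles equipping and dealing melee hit damage.
; On equip it attaches to the hand or stow socket by combat state, registers with the owner's CombatComponent and sends its combat type to the AnimInstance.
; Its collision component traces the item mesh, ignoring the owner, and hits apply point damage to actors that accept it.
; SimulateWeaponPhysics sets the PhysicsActor profile but passes false to SetSimulatePhysics.
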(event OnHit(MainWeaponCollisionComponent)
  (params (HitResult :type Hit%20Result%20Structure))
  (bind _hitactor (Collision|BreakHitResult HitResult))
  (bind _returnvalue (Class|CombatBPI|CanRecieveDamage(Message) _hitactor))
  (if _returnvalue
    (Game|Damage|ApplyPointDamage _hitactor (Variables|Default|GetDamage) (Transformation|GetActorForwardVector (Components|GetOwner)) HitResult (Game|GetInstigatorController) self)))

(event Custom|SimulateWeaponPhysics
  (bind _mesh (CallFunction|GetItemMesh))
  (Collision|SetCollisionProfileName _mesh "PhysicsActor" true :!class /Script/Engine.PrimitiveComponent)
  (Physics|SetSimulatePhysics _mesh false))

(event EventBeginPlay
  (|CallParentFunction) ; This node is disabled and will not be called.\nDrag off pins to build functionality.
)

(event Collision|EventActorBeginOverlap
  (params (OtherActor :type Actor%20Object%20Reference))
  (|CallParentFunction OtherActor) ; This node is disabled and will not be called.\nDrag off pins to build functionality.
)

(event EventTick
  (params (DeltaSeconds :type Float%20%28single-precision%29))
  (|CallParentFunction DeltaSeconds) ; This node is disabled and will not be called.\nDrag off pins to build functionality.
)

(fn ConstructionScript
  (|CallParentFunction))

(fn OnEquipped
  (Variables|Default|SetCombatCombatComponent (Actor|GetComponentbyClass (Components|GetOwner) "/Game/CombatSystem/Blueprints/Components/CombatComponent.CombatComponent_C"))
  (CallFunction|AttachActor (select (Default|IsCombatEnabled? (Variables|Default|GetCombatCombatComponent)) (Variables|Initialization|GetHandSocketName) (Variables|Default|GetAttach%20Socket%20Name)))
  (Default|SetMainWeapon (Variables|Default|GetCombatCombatComponent) self)
  (Class|AnimInstanceBPI|UpdateCombatType(Message) (Components|SkeletalMesh|GetAnimInstance (Variables|/Script/Engine.Character|GetMesh (.AsCharacter (Utilities|Casting|CastToCharacter (Components|GetOwner))))) (Variables|Initialization|GetCombatType))
  (Default|SetCollisionMesh (Variables|Default|GetMainWeaponCollisionComponent) (CallFunction|GetItemMesh))
  (Default|AddActortoIgnore (Variables|Default|GetMainWeaponCollisionComponent) (Components|GetOwner)))