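; BP_MasterPose is a wearable equipment actor for skinned gear that follows the owning character's animation and contributes an armor value.
; AttachActor snaps its item skeletal mesh to a socket on the character mesh and sets that mesh as master pose component.
; OnEquipped and OnUnequipped extend the parent logic, adding and then subtracting ArmorValue through the owner's BP_StatsComponent.
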(event EventBeginPlay
  (|CallParentFunction) ; This node is disabled and will not be called.\nDrag off pins to build functionality.
)

(event Collision|EventActorBeginOverlap
  (params (OtherActor :type Actor%20Object%20Reference))
  (|CallParentFunction OtherActor) ; This node is disabled and will not be called.\nDrag off pins to build functionality.
)

(event EventTick
  (params (DeltaSeconds :type Float%20%28single-precision%29))
  (|CallParentFunction DeltaSeconds) ; This node is disabled and will not be called.\nDrag off pins to build functionality.
)

(fn ConstructionScript
  (|CallParentFunction))

(fn AttachActor
  (params (SocketName :type Name :default "None"))
  (bind _returnvalue (Components|GetOwner))
  (bind _ascharacter (Utilities|Casting|CastToCharacter _returnvalue))
  (bind _mesh (Variables|/Script/Engine.Character|GetMesh _ascharacter))
  (Utilities|IsValid (Variables|/Script/Engine.SkinnedMeshComponent|GetSkeletalMesh (Variables|Default|GetitemSkeletalMesh))
    (:Is%20Valid
      (Transformation|AttachComponentToComponent (Variables|Default|GetitemSkeletalMesh) _mesh SocketName "SnapToTarget" "SnapToTarget" "SnapToTarget" true)
      (Class|SkinnedMeshComponent|SetMasterPoseComponent (Variables|Default|GetitemSkeletalMesh) _mesh false)
      (return))
    (:Is%20Not%20Valid
      (return))))

(fn OnEquipped
  (|CallParentFunction)
  (Default|ModifyCurrentStatsValue (Actor|GetComponentbyClass (Components|GetOwner) "/Game/CombatSystem/Blueprints/Components/BP_StatsComponent.BP_StatsComponent_C") (Variables|Stats|GetArmorValue) "NewEnumerator3" false))

(fn OnUnequipped
  (|CallParentFunction)
  (Default|ModifyCurrentStatsValue (Actor|GetComponentbyClass (Components|GetOwner) "/Game/CombatSystem/Blueprints/Components/BP_StatsComponent.BP_StatsComponent_C") (* (Variables|Stats|GetArmorValue) -1.0) "NewEnumerator3" false))